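; Door that opens once its red, blue and green indicator lights are all lit.
; LightColorDoor compares the incoming color to red, then blue, by RGB distance against a threshold, falling back to green for anything else.
; Each match tints that light's dynamic pulse material, created in the construction script.
; When all three are lit, a timeline lerps the actor's Z from its construction-time position to DoorEndPoint.
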(event EventBeginPlay)

(event EventActorBeginOverlap
  (params (OtherActor :type Actor%20Object%20Reference)))

(event EventTick
  (params (DeltaSeconds :type Float%20%28single-precision%29)))

(event EventLightColorDoor
  (params (Color :type Linear%20Color%20Structure))
  (bind _doorstartpoint (Variables|Default|GetDoorStartPoint))
  (Utilities|FlowControl|Sequence
    (:then_0
      ;[1 1 1] turn on light
      (bind _difference (CallFunction|GetColorDifference Color (Variables|Default|GetRedColor)))
      (if (< _difference (Variables|Default|GetColorThreshold))
        (Rendering|Material|SetVectorParameterValue (Variables|Default|GetRedLightMaterial) "PulseColor" (Variables|Default|GetRedColor) :!class /Script/Engine.MaterialInstanceDynamic)
        (Variables|Default|SetIsRedLit true)
        (else
          (bind _difference_2 (CallFunction|GetColorDifference Color (Variables|Default|GetBlueColor)))
          (if (< _difference_2 (Variables|Default|GetColorThreshold))
            (Rendering|Material|SetVectorParameterValue (Variables|Default|GetBlueLightMaterial) "PulseColor" (Variables|Default|GetBlueColor) :!class /Script/Engine.MaterialInstanceDynamic)
            (Variables|Default|SetIsBlueLit true)
            (else
              (Rendering|Material|SetVectorParameterValue (Variables|Default|GetGreenLightMaterial) "PulseColor" (Variables|Default|GetGreenColor) :!class /Script/Engine.MaterialInstanceDynamic)
              (Variables|Default|SetIsGreenLit true))))))
    (:then_1
      (if (Math|Boolean|ANDBoolean (Variables|Default|GetIsRedLit) (Variables|Default|GetIsGreenLit) (Variables|Default|GetIsBlueLit))
        (bind _opendoor (Timeline|ColorDoor_Open Play)
          (:Update
            (Transformation|SetActorLocation (Math|Vector|MakeVector (.x _doorstartpoint) (.y _doorstartpoint) (Math|Float|Lerp (.z _doorstartpoint) (.z (Variables|Default|GetDoorEndPoint)) _opendoor)) false)))))))

(fn ConstructionScript
  (bind _initialcolor (Variables|Default|GetInitialColor))
  (Utilities|FlowControl|Sequence
    (:then_0
      (bind _returnvalue (Rendering|Material|CreateDynamicMaterialInstance (Variables|Default|GetRedLight) 0 "/Game/Materials/M_Tech_Hex_Tile_Pulse_With_Color.M_Tech_Hex_Tile_Pulse_With_Color" :!class /Script/Engine.PrimitiveComponent))
      (bind _output_get (Variables|Default|SetRedLightMaterial _returnvalue))
      (Rendering|Material|SetVectorParameterValue _output_get "PulseColor" _initialcolor :!class /Script/Engine.MaterialInstanceDynamic))
    (:then_1
      (bind _returnvalue_2 (Rendering|Material|CreateDynamicMaterialInstance (Variables|Default|GetBlueLight) 0 "/Game/Materials/M_Tech_Hex_Tile_Pulse_With_Color.M_Tech_Hex_Tile_Pulse_With_Color" :!class /Script/Engine.PrimitiveComponent))
      (bind _output_get_2 (Variables|Default|SetBlueLightMaterial _returnvalue_2))
      (Rendering|Material|SetVectorParameterValue _output_get_2 "PulseColor" _initialcolor :!class /Script/Engine.MaterialInstanceDynamic))
    (:then_2
      (bind _returnvalue_3 (Rendering|Material|CreateDynamicMaterialInstance (Variables|Default|GetGreenLight) 0 "/Game/Materials/M_Tech_Hex_Tile_Pulse_With_Color.M_Tech_Hex_Tile_Pulse_With_Color" :!class /Script/Engine.PrimitiveComponent))
      (bind _output_get_3 (Variables|Default|SetGreenLightMaterial _returnvalue_3))
      (Rendering|Material|SetVectorParameterValue _output_get_3 "PulseColor" _initialcolor :!class /Script/Engine.MaterialInstanceDynamic))
    (:then_3
      (Variables|Default|SetDoorStartPoint (Transformation|GetActorLocation)))))

(fn TurnonLight
  (params (Color :type Linear%20Color%20Structure) (Material :type Material%20Instance%20Dynamic%20Object%20Reference))
  (Rendering|Material|SetVectorParameterValue Material "None" Color :!class /Script/Engine.MaterialInstanceDynamic))

(fn GetColorDifference
  (params (Color1 :type Linear%20Color%20Structure) (Color2 :type Linear%20Color%20Structure))
  (return (Math|Float|Sqrt (Math|Vector|VectorLengthSquared (- (Math|Conversions|ToVector(LinearColor) Color1) (Math|Conversions|ToVector(LinearColor) Color2))))))